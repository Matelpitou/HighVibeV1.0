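; Ranged enemy character that chases the player, then stops to throw projectiles.
; Tick drives it: beyond range it uses AIMoveTo, within range a timeline adjusts walk speed before Shoot, and it yaws toward the player while shooting or cooling down.
; The throw montage's notify spawns BP_ProjED pitched upward, followed by a delay-based cooldown.
; HitTaken handles damage, player combo, hit reaction and death; an older death chain is left unconnected.
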(event Custom|Focus%20player
  (if (> (Transformation|GetDistanceTo self (Variables|Default|GetTPC)) 6e+02)
    (Variables|/Script/Engine.CharacterMovementComponent|SetMaxWalkSpeed (Variables|Character|GetCharacterMovement) 3e+02)
    (AI|AIMoveTo self (Transformation|GetWorldLocation (Variables|/Script/Engine.Character|GetMesh (Variables|Default|GetTPC))) 0 5.0 false)
    (else
      (CallFunction|StartShooting))))

(event Custom|Start%20shooting
  (Variables|Default|Setshooting true)
  (Utilities|FlowControl|DoOnce false
    (:Completed
      (if (> (Variables|/Script/Engine.CharacterMovementComponent|GetMaxWalkSpeed (Variables|Character|GetCharacterMovement)) 1e+01)
        (bind _speed (Timeline|Timeline PlayFromStart)
          (:Update
            (Variables|/Script/Engine.CharacterMovementComponent|SetMaxWalkSpeed (Variables|Character|GetCharacterMovement) _speed))
          (:Finished
            (CallFunction|Shoot :!label _label)))
        (else
          (goto _label))))))

(event Custom|Shoot
  (bind _capsulecomponent (Variables|Default|GetCapsuleComponent))
  (bind _returnvalue (Transformation|GetWorldTransform _capsulecomponent))
  (if (Variables|Default|GetCooldown)
    (Utilities|FlowControl|Sequence
      (:then_0
        (Animation|Montage|PlayMontage (Variables|Character|GetMesh) "/Game/EnnemiTest/EnnemiTest2/EnnemiDistance/AM_ThrowED.AM_ThrowED"
          (:OnCompleted
            (Variables|Default|Setshooting false :!label _label)
            (Utilities|FlowControl|DoOnce false) ; enters at Reset
          )
          (:OnInterrupted
            (goto _label))
          (:OnNotifyBegin
            (bind _returnvalue_2 (Game|SpawnActorfromClass "/Game/EnnemiTest/EnnemiTest2/EnnemiDistance/BP_ProjED.BP_ProjED_C" (Math|Transform|MakeTransform (.location _returnvalue) (Math|Rotator|MakeRotator (.roll (.rotation _returnvalue)) (+ (.pitch (.rotation _returnvalue)) 6e+01) (.yaw (.rotation _returnvalue))) (.scale _returnvalue)) "Undefined" "MultiplyWithRoot" 0 0))
            (Default|CTipar _returnvalue_2 self))))
      (:then_1
        (Variables|Default|SetCooldown false)
        (Utilities|FlowControl|Delay 5.0)
        (Variables|Default|SetCooldown true)))
    (else
      (Variables|Default|Setshooting false)
      (Utilities|FlowControl|DoOnce false) ; enters at Reset
    )))

(event EventBeginPlay
  (|CallParentFunction)
  (Variables|Default|SetMax%20Walk%20Speed (Variables|/Script/Engine.CharacterMovementComponent|GetMaxWalkSpeed (Variables|Character|GetCharacterMovement)))
  (bind _asbp_third_person_character (Utilities|Casting|CastToBP_ThirdPersonCharacter (Game|GetPlayerCharacter 0)))
  (Variables|Default|SetTPC _asbp_third_person_character))

(event EventHitTaken
  (params (Damage :type Float%20%28double-precision%29) (AugmentCombo :type Boolean))
  (bind _charactermovement (Variables|Character|GetCharacterMovement))
  (bind _output_get (Variables|Default|SetHP (- (Variables|Default|GetHP) Damage)))
  (if (<= _output_get 0.0)
    (CallFunction|DeathEnnemi)
    (Utilities|FlowControl|Sequence
      (:then_0
        (Animation|Montage|PlayMontage (Variables|Character|GetMesh) "/Game/EnnemiTest/EnnemiTest2/EnnemiDistance/AM_MortED.AM_MortED"
          (:OnBlendOut
            _)
          (:OnInterrupted
            _))
        (Components|Animation|PlayAnimation (Variables|Character|GetMesh) "/Game/EnnemiTest/EnnemiTest2/A_Ennemi2MortLoop.A_Ennemi2MortLoop" true))
      (:then_1
        (Utilities|FlowControl|Delay 5.0)
        (Actor|DestroyActor)))
    (else
      (if AugmentCombo
        (Default|AugmentCombo (Variables|Default|GetTPC) 1))
      (Variables|Default|SetSeFaitTaper true)
      (Animation|Montage|PlayMontage (Variables|Character|GetMesh) "/Game/EnnemiTest/EnnemiTest2/AM_Ennemi2TakeHit.AM_Ennemi2TakeHit" 2.0
        (:then
          (Variables|/Script/Engine.CharacterMovementComponent|SetMaxWalkSpeed _charactermovement 0.0))
        (:OnCompleted
          (Variables|Default|SetSeFaitTaper false)
          (Variables|/Script/Engine.CharacterMovementComponent|SetMaxWalkSpeed _charactermovement (Variables|Default|GetMax%20Walk%20Speed)))))))

(event EventTick
  (params (DeltaSeconds :type Float%20%28single-precision%29))
  (bind _capsulecomponent (Variables|Default|GetCapsuleComponent))
  (bind _returnvalue (Transformation|GetWorldRotation _capsulecomponent))
  (if (not (Variables|Default|GetMort))
    (if (Variables|Default|Getshooting)
      (Transformation|SetActorRotation self (Math|Rotator|MakeRotator (.roll _returnvalue) (.pitch _returnvalue) (.yaw (Math|Rotator|FindLookatRotation (Transformation|GetWorldLocation (Variables|Default|GetCapsuleComponent)) (Transformation|GetWorldLocation (Variables|/Script/Engine.Character|GetMesh (Variables|Default|GetTPC)))))) :!label _label)
      (elif (Variables|Default|GetCooldown)
        (if (not (Variables|Default|GetIdlePause))
          (CallFunction|FocusPlayer))
        (else
          (goto _label))))))

(fn ConstructionScript
  (|CallParentFunction))