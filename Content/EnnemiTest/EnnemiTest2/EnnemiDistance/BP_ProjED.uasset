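; BP_ProjED is a projectile for the ranged enemy BP_EnnemiD that damages the player.
; CTipar takes the enemy, then impulses the Cylinder along the root's forward vector, scaled by a ballistic range formula using enemy-to-player distance and a fixed launch angle.
; When the Cylinder overlaps BP_ThirdPersonCharacter, it calls TakeHit with fixed damage and destroys itself.
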(event OnComponentBeginOverlap(Cylinder)
  (params (OverlappedComponent :type Primitive%20Component%20Object%20Reference) (OtherActor :type Actor%20Object%20Reference) (OtherComp :type Primitive%20Component%20Object%20Reference) (OtherBodyIndex :type Integer) (bFromSweep :type Boolean) (SweepResult :type Hit%20Result%20Structure%20%28by%20ref%29))
  (bind _asbp_third_person_character (Utilities|Casting|CastToBP_ThirdPersonCharacter OtherActor))
  (Default|TakeHit _asbp_third_person_character 8.0)
  (Actor|DestroyActor))

(event Custom|CTipar
  (params (NewParam :type Actor%20Object%20Reference))
  (bind _asbp_ennemi_d (Utilities|Casting|CastToBP_EnnemiD NewParam))
  (bind _output_get (Variables|Default|SetAs%20BP%20Ennemi%20D _asbp_ennemi_d))
  (Variables|Default|SetEnnemiePosition (Transformation|GetWorldLocation (Variables|/Script/Engine.Character|GetCapsuleComponent _output_get)))
  (bind _asbp_third_person_character (Utilities|Casting|CastToBP_ThirdPersonCharacter (Game|GetPlayerCharacter 0)))
  (bind _output_get_2 (Variables|Default|SetAs%20BP%20Third%20Person%20Character _asbp_third_person_character))
  (Variables|Default|SetPlayerPosition (Transformation|GetWorldLocation (Variables|/Script/Engine.Character|GetCapsuleComponent _output_get_2)))
  (Physics|AddImpulse (Variables|Default|GetCylinder) (* (* (Math|Float|Sqrt (* (/ (Math|Vector|Distance(Vector) (Variables|Default|GetPlayerPosition) (Variables|Default|GetEnnemiePosition)) (Math|Trig|Sin(Degrees) 1.2e+02)) 9.81)) 155.0) (Math|Vector|GetForwardVector (Transformation|GetWorldRotation (Variables|Default|GetDefaultSceneRoot)))) "None" false))

(fn ConstructionScript)