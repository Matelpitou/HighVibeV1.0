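; Elite enemy AI that hunts the third-person player and picks an attack by distance.
; When idle, Tick selects close melee, a mid-range leap (randomly swapped for melee), a sped-up charge into a kick, or plain pursuit.
; The leap follows a spawned spline and damages by landing proximity, while melee and kick use sphere traces.
; HitTaken lowers HP, feeds the player's combo, and handles death animation and delayed destruction.
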(event Custom|SelectInstruction
  (params (DistanceToPlayer :type Float%20%28double-precision%29))
  (Variables|Default|SetPasInstruction false)
  (if (Math|Float|InRange(Float) DistanceToPlayer 0.0 5e+02)
    (CallFunction|PrepCoupProche)
    (elif (Math|Float|InRange(Float) DistanceToPlayer 5e+02 1.5e+03 false)
      (CallFunction|PrepBoom)
      (elif (Math|Float|InRange(Float) DistanceToPlayer 1.5e+03 2e+03 false)
        (CallFunction|PrepCharge)
        (else
          (CallFunction|TropLoin))))))

(event Custom|PrepCharge
  (bind _returnvalue (Transformation|GetActorLocation))
  ;[1 1 1] Charge
  (Animation|Montage|PlayMontage (Variables|Character|GetMesh) "/Game/EnnemiTest/EnnemiTest2/EnnemiElite/AM_ElanEnnemiElite.AM_ElanEnnemiElite"
    (:OnCompleted
      (Variables|/Script/Engine.CharacterMovementComponent|SetMaxWalkSpeed (Variables|Character|GetCharacterMovement) 8e+02)
      (Variables|Default|SetCharging true)
      (AI|AIMoveTo self (Transformation|GetActorLocation (Variables|Default|GetTPC)) 0 3e+02 false :!label _label
        (:then
          (if (> (Transformation|GetDistanceTo self (Variables|Default|GetTPC)) 5e+02)
            (Utilities|FlowControl|Delay (Utilities|Time|GetWorldDeltaSeconds))
            (goto _label)))
        (:OnSuccess
          (Animation|Montage|PlayMontage (Variables|Character|GetMesh) "/Game/EnnemiTest/EnnemiTest2/EnnemiElite/AM_KickElite.AM_KickElite"
            (:then
              (Utilities|FlowControl|DoOnce false :!label _label_2
                (:Completed
                  (bind _outhits (Collision|MultiSphereTraceByChannel _returnvalue (+ _returnvalue (* (Transformation|GetActorForwardVector) 320)) 8e+01 "TraceTypeQuery1" false 0 "ForDuration"))
                  (for _array_element _outhits
                    (bind _asbp_third_person_character (Utilities|Casting|CastToBP_ThirdPersonCharacter (.HitActor (Collision|BreakHitResult _array_element))))
                    (Default|TakeHit _asbp_third_person_character 2e+01)))))
            (:OnCompleted
              (Utilities|FlowControl|Delay 0.2)
              (Variables|Default|SetCharging false)
              (Variables|Default|SetPasInstruction true)
              (Variables|/Script/Engine.CharacterMovementComponent|SetMaxWalkSpeed (Variables|Character|GetCharacterMovement) 6e+02)
              (goto _label_2 Reset))))))))

(event Custom|PrepBoom
  (bind _tpc (Variables|Default|GetTPC))
  ;[1 1 1] Boom
  (if (== (Math|Random|RandomIntegerinRange 0 2) 0)
    (Animation|Montage|PlayMontage (Variables|Character|GetMesh) "/Game/EnnemiTest/EnnemiTest2/EnnemiElite/AM_ElanEnnemiElite.AM_ElanEnnemiElite"
      (:OnCompleted
        (Utilities|FlowControl|Sequence
          (:then_0
            (Transformation|SetActorRotation (Math|Rotator|FindLookatRotation (Transformation|GetActorLocation self) (Transformation|GetWorldLocation (Variables|/Script/Engine.Character|GetCapsuleComponent (Variables|Default|GetTPC)))))
            (bind _returnvalue (Game|SpawnActorfromClass "/Game/EnnemiTest/EnnemiTest2/EnnemiElite/BP_Spline.BP_Spline_C" (Transformation|GetWorldTransform (Variables|Default|GetCapsuleComponent)) "Undefined" "MultiplyWithRoot" 0 0))
            (Variables|Default|SetSplineActor _returnvalue)
            (Spline|SetLocationatSplinePoint (Variables|/Game/EnnemiTest/EnnemiTest2/EnnemiElite/BP_Spline.BP_Spline_C|GetSpline (Variables|Default|GetSplineActor)) 1 (Transformation|GetWorldLocation (Variables|/Script/Engine.Character|GetCapsuleComponent (Variables|Default|GetTPC))) "World" true)
            (Spline|SetTangentsatSplinePoint (Variables|/Game/EnnemiTest/EnnemiTest2/EnnemiElite/BP_Spline.BP_Spline_C|GetSpline (Variables|Default|GetSplineActor)) 1 (Math|Vector|MakeVector (* (Spline|GetSplineLength (Variables|/Game/EnnemiTest/EnnemiTest2/EnnemiElite/BP_Spline.BP_Spline_C|GetSpline (Variables|Default|GetSplineActor))) 1.2) 0.0 (* (Spline|GetSplineLength (Variables|/Game/EnnemiTest/EnnemiTest2/EnnemiElite/BP_Spline.BP_Spline_C|GetSpline (Variables|Default|GetSplineActor))) -2.0)) (Math|Vector|MakeVector (* (Spline|GetSplineLength (Variables|/Game/EnnemiTest/EnnemiTest2/EnnemiElite/BP_Spline.BP_Spline_C|GetSpline (Variables|Default|GetSplineActor))) 1.2) 0.0 (* (Spline|GetSplineLength (Variables|/Game/EnnemiTest/EnnemiTest2/EnnemiElite/BP_Spline.BP_Spline_C|GetSpline (Variables|Default|GetSplineActor))) -2.0)) "Local" true)
            (bind _newtrack_0 (Timeline|Timeline_0 PlayFromStart)
              (:Update
                (Transformation|SetWorldLocation (Variables|Default|GetCapsuleComponent) (Spline|GetLocationatDistanceAlongSpline (Variables|/Game/EnnemiTest/EnnemiTest2/EnnemiElite/BP_Spline.BP_Spline_C|GetSpline (Variables|Default|GetSplineActor)) (Math|Float|Lerp 0.0 (Spline|GetSplineLength (Variables|/Game/EnnemiTest/EnnemiTest2/EnnemiElite/BP_Spline.BP_Spline_C|GetSpline (Variables|Default|GetSplineActor))) _newtrack_0) "World") false false))
              (:Finished
                (if (< (Math|Vector|Distance(Vector) (Transformation|GetActorLocation) (Transformation|GetActorLocation _tpc)) 3e+02)
                  (Default|TakeHit _tpc 2e+01)))))
          (:then_1
            (Animation|Montage|PlayMontage (Variables|Character|GetMesh) "/Game/EnnemiTest/EnnemiTest2/EnnemiElite/AM_JumpElite.AM_JumpElite"
              (:OnCompleted
                (Variables|Default|SetJumping true)
                (Utilities|FlowControl|DoOnce false :!label _label
                  (:Completed
                    (bind _newtrack_0_2 (Timeline|Timeline PlayFromStart)
                      (:Update
                        (Variables|Default|SetJumpState _newtrack_0_2))
                      (:Finished
                        (Utilities|FlowControl|Sequence
                          (:then_0
                            (goto _label Reset))
                          (:then_1
                            (Variables|Default|SetJumping false)
                            (Variables|Default|SetPasInstruction true)))))))))))))
    (else
      (CallFunction|PrepCoupProche))))

(event Custom|PrepCoupProche
  (bind _returnvalue (Transformation|GetActorLocation))
  ;[1 1 1] CoupProche
  (AI|AIMoveTo self (Transformation|GetActorLocation (Variables|Default|GetTPC)) 0 5.0 false :!label _label
    (:then
      (Utilities|FlowControl|Delay (Utilities|Time|GetWorldDeltaSeconds))
      (if (> (Transformation|GetDistanceTo self (Variables|Default|GetTPC)) 3e+02)
        (goto _label)
        (else
          (Animation|Montage|PlayMontage (Variables|Character|GetMesh) "/Game/EnnemiTest/EnnemiTest2/EnnemiElite/A_CoupProcheElite.A_CoupProcheElite"
            (:OnCompleted
              (Variables|Default|SetPasInstruction true))
            (:OnNotifyBegin
              (bind _outhits (Collision|MultiSphereTraceByChannel _returnvalue (+ _returnvalue (* (Transformation|GetActorForwardVector) 150)) 5e+01 "TraceTypeQuery1" false 0 "Persistent"))
              (for _array_element _outhits
                (bind _asbp_third_person_character (Utilities|Casting|CastToBP_ThirdPersonCharacter (.HitActor (Collision|BreakHitResult _array_element))))
                (Default|TakeHit _asbp_third_person_character 15.0)))))))))

(event Custom|TropLoin
  ;[1 1 1] Trop loin de la cible
  (Variables|Default|SetPasInstruction true)
  (AI|AIMoveTo self (Transformation|GetActorLocation (Variables|Default|GetTPC)) 0 5.0 false))

(event EventTick
  (params (DeltaSeconds :type Float%20%28single-precision%29))
  (Utilities|FlowControl|Gate false :!label _label
    (:Exit
      (if (Variables|Default|GetMort)
        (goto _label Close)
        (elif (not (Variables|Default|GetIdlePause))
          (if (Variables|Default|GetPasInstruction)
            (bind _output_get (Variables|Default|SetDistance (Transformation|GetDistanceTo self (Variables|Default|GetTPC))))
            (CallFunction|SelectInstruction _output_get)))))))

(event EventBeginPlay
  (|CallParentFunction)
  (bind _asbp_third_person_character (Utilities|Casting|CastToBP_ThirdPersonCharacter (Game|GetPlayerCharacter 0)))
  (Variables|Default|SetTPC _asbp_third_person_character))

(event EventBumpElite
  ;[1 1 1] KnockElite
)

(event EventHitTaken
  (params (Damage :type Float%20%28double-precision%29) (AugmentCombo :type Boolean))
  ;[1 1 1] Hit Normal
  (bind _output_get (Variables|Default|SetHP (- (Variables|Default|GetHP) Damage)))
  (if (<= _output_get 0.0)
    (CallFunction|DeathEnnemi)
    (Utilities|FlowControl|Sequence
      (:then_0
        (Animation|Montage|PlayMontage (Variables|Character|GetMesh) "/Game/EnnemiTest/EnnemiTest2/EnnemiElite/AM_MortElite2.AM_MortElite2"
          (:OnBlendOut
            _)
          (:OnInterrupted
            _))
        (Components|Animation|PlayAnimation (Variables|Character|GetMesh) "/Game/EnnemiTest/EnnemiTest2/A_Ennemi2MortLoop.A_Ennemi2MortLoop" true))
      (:then_1
        (Utilities|FlowControl|Delay 5.0)
        (Actor|DestroyActor)))
    (else
      (if AugmentCombo
        (Default|AugmentCombo (Variables|Default|GetTPC) 1))
      (Variables|Default|SetSeFaitTaper true)
      (Variables|Default|SetSeFaitTaper false)
      (Variables|/Script/Engine.CharacterMovementComponent|SetMaxWalkSpeed (Variables|Character|GetCharacterMovement) (Variables|Default|GetMax%20Walk%20Speed)))))

(fn ConstructionScript
  (|CallParentFunction))