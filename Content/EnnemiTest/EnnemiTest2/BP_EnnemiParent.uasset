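; Base enemy Blueprint that registers itself in the game mode's AllEnnemi list and starts at full HP.
; A self-recalling one-frame delay loop syncs the mesh's depth and custom-depth rendering to the Grabble flag.
; HitTaken and BumpElite are empty hooks, while SlowTime resets time dilation to normal unless the game mode's slow-time is active.
; DeathEnnemi flags death, then once adjusts capsule collision, zeroes walk speed and unregisters the enemy.
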(event Custom|HitTaken
  (params (Damage :type Float%20%28double-precision%29) (AugmentCombo :type Boolean)))

(event Custom|BumpElite)

(event Custom|IsGrabble?
  (bind _mesh (Variables|Character|GetMesh))
  (if (Variables|Default|GetGrabble?)
    (Class|PrimitiveComponent|SetRenderinDepthPass _mesh true)
    (Rendering|SetRenderCustomDepth _mesh true)
    (else
      (Class|PrimitiveComponent|SetRenderinDepthPass _mesh false)
      (Rendering|SetRenderCustomDepth _mesh false)))
  (Utilities|FlowControl|Delay (Utilities|Time|GetWorldDeltaSeconds))
  (CallFunction|IsGrabble?))

(event Custom|SlowTime
  (if (Variables|/Game/ThirdPerson/Blueprints/BP_ThirdPersonGameMode.BP_ThirdPersonGameMode_C|GetSlowTime? (Variables|Default|GetGm))
    (Variables|Default|SetCustomTimeDilation (Variables|Default|GetCustom%20Time%20Dilation))
    (else
      (Variables|Default|SetCustomTimeDilation 1.0))))

(event EventBeginPlay
  (bind _asbp_third_person_game_mode (Utilities|Casting|CastToBP_ThirdPersonGameMode (Game|GetGameMode)))
  (bind _output_get (Variables|Default|SetGm _asbp_third_person_game_mode))
  (Utilities|Array|Add (Variables|/Game/ThirdPerson/Blueprints/BP_ThirdPersonGameMode.BP_ThirdPersonGameMode_C|GetAllEnnemi _output_get) self)
  (CallFunction|IsGrabble?)
  (Variables|Default|SetHP (Variables|Default|GetHPMax)))

(fn ConstructionScript)

(fn DeathEnnemi
  (Variables|Default|SetMort true)
  (Utilities|FlowControl|DoOnce false
    (:Completed
      (Collision|SetCollisionResponsetoChannel (Variables|Collision|GetCapsuleComponent) "ECC_GameTraceChannel2" "ECR_Ignore")
      (Collision|SetCollisionEnabled (Variables|Collision|GetCapsuleComponent) "PhysicsOnly")
      (Variables|/Script/Engine.CharacterMovementComponent|SetMaxWalkSpeed (Variables|Character|GetCharacterMovement) 0.0)
      (Utilities|Array|RemoveItem (Variables|/Game/ThirdPerson/Blueprints/BP_ThirdPersonGameMode.BP_ThirdPersonGameMode_C|GetAllEnnemi (Variables|Default|GetGm)) self))))