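; Breakable parking meter (parcmètre) that drops BP_Money when it receives EnviroHit.
; Each accepted hit spawns money at SpawnMoney and plays a scale timeline on Base, then decrements HP, which starts at HPMax.
; A DoOnce gate ignores further hits until that animation finishes.
; At zero HP, a second scale timeline plays, then the meter spawns a final money pickup and destroys itself.
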(event EventEnviroHit
  (params (PlayerRotation :type Rotator :default "0, 0, 0"))
  (bind _hp (Variables|Default|GetHP))
  (Utilities|FlowControl|DoOnce false :!label _label
    (:Completed
      (Game|SpawnActorfromClass "/Game/InteractionsEnviro/BP_Money.BP_Money_C" (Math|Transform|MakeTransform (Transformation|GetWorldLocation (Variables|Default|GetSpawnMoney)) "0, 0, 0" "1.000000,1.000000,1.000000") "Undefined" "MultiplyWithRoot" 0 0)
      (bind _newtrack_0 (Timeline|Scale PlayFromStart)
        (:Update
          (Transformation|SetWorldScale3D (Variables|Default|GetBase) (Math|Vector|MakeVector (.x _newtrack_0) (.y _newtrack_0) (.z _newtrack_0))))
        (:Finished
          (Math|Integer|DecrementInt _hp
            (:%20%20
              (if (<= _hp 0)
                (bind _newtrack_0_2 (Timeline|Timeline PlayFromStart)
                  (:Update
                    (Transformation|SetWorldScale3D (Variables|Default|GetBase) (Math|Vector|MakeVector (.x _newtrack_0_2) (.y _newtrack_0_2) (.z _newtrack_0_2))))
                  (:Finished
                    (Game|SpawnActorfromClass "/Game/InteractionsEnviro/BP_Money.BP_Money_C" (Math|Transform|MakeTransform (Transformation|GetWorldLocation (Variables|Default|GetBase)) "0, 0, 0" "1.000000,1.000000,1.000000") "Undefined" "MultiplyWithRoot" 0 0)
                    (Actor|DestroyActor)))
                (else
                  (goto _label Reset))))))))))

(event EventBeginPlay
  (Variables|Default|SetHP (Variables|Default|GetHPMax)))

(fn ConstructionScript)