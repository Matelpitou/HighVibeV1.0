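; BP_Jerrican is an interactive environment prop that gets launched when hit and explodes, damaging nearby enemies.
; EnviroHit enables physics on the cube and shoves it along the player's facing direction, arming it.
; It detonates after a short delay, or on any Box overlap once armed.
; Detonation sphere-traces for BP_EnnemiParent actors to damage without adding combo, spawns BP_AOE_Jerrican, then destroys itself.
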(event OnComponentBeginOverlap(Box)
  (params (OverlappedComponent :type Primitive%20Component%20Object%20Reference) (OtherActor :type Actor%20Object%20Reference) (OtherComp :type Primitive%20Component%20Object%20Reference) (OtherBodyIndex :type Integer) (bFromSweep :type Boolean) (SweepResult :type Hit%20Result%20Structure%20%28by%20ref%29))
  (bind _cube (Variables|Default|GetCube))
  (bind _returnvalue (Transformation|GetWorldLocation _cube))
  (if (Variables|Default|GetTriggered)
    (bind _outhits (Collision|MultiSphereTraceByChannel _returnvalue _returnvalue 3.5e+02 "TraceTypeQuery1" false 0 "ForDuration"))
    (Utilities|FlowControl|Sequence
      (:then_0
        (for _array_element _outhits
          (bind _asbp_ennemi_parent (Utilities|Casting|CastToBP_EnnemiParent (.HitActor (Collision|BreakHitResult _array_element))))
          (Default|HitTaken _asbp_ennemi_parent (Variables|Default|GetDamage) false)))
      (:then_1
        (Game|SpawnActorfromClass "/Game/InteractionsEnviro/BP_AOE_Jerrican.BP_AOE_Jerrican_C" (Math|Transform|MakeTransform (Transformation|GetWorldLocation (Variables|Default|GetCube)) "0, 0, 0" "1.000000,1.000000,1.000000") "Undefined" "MultiplyWithRoot" 0 0)
        (Utilities|FlowControl|Delay 0.2)
        (Actor|DestroyActor)))))

(event EventBeginPlay)

(event Collision|EventActorBeginOverlap
  (params (OtherActor :type Actor%20Object%20Reference)))

(event EventTick
  (params (DeltaSeconds :type Float%20%28single-precision%29)))

(event EventEnviroHit
  (params (PlayerRotation :type Rotator :default "0, 0, 0"))
  (bind _cube (Variables|Default|GetCube))
  (bind _returnvalue (Transformation|GetWorldLocation _cube))
  (Physics|SetSimulatePhysics (Variables|Default|GetCube) true)
  (Physics|AddImpulse (Variables|Default|GetCube) (* (Math|Vector|GetForwardVector PlayerRotation) 8e+03) "None" false)
  (Variables|Default|SetTriggered true)
  (Utilities|FlowControl|Delay 2.0)
  (bind _outhits (Collision|MultiSphereTraceByChannel _returnvalue _returnvalue 3.5e+02 "TraceTypeQuery1" false 0 "ForDuration"))
  (Utilities|FlowControl|Sequence
    (:then_0
      (for _array_element _outhits
        (bind _asbp_ennemi_parent (Utilities|Casting|CastToBP_EnnemiParent (.HitActor (Collision|BreakHitResult _array_element))))
        (Default|HitTaken _asbp_ennemi_parent (Variables|Default|GetDamage) false)))
    (:then_1
      (Game|SpawnActorfromClass "/Game/InteractionsEnviro/BP_AOE_Jerrican.BP_AOE_Jerrican_C" (Math|Transform|MakeTransform (Transformation|GetWorldLocation (Variables|Default|GetCube)) "0, 0, 0" "1.000000,1.000000,1.000000") "Undefined" "MultiplyWithRoot" 0 0)
      (Utilities|FlowControl|Delay 0.2)
      (Actor|DestroyActor))))

(fn ConstructionScript)