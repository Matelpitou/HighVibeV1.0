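; Burning barrel environment prop that, when hit, tips over once and creates a temporary fire zone that damages enemies.
; EnviroHit orients the actor from the player's rotation with yaw flipped, then a timeline pitches the Sphere before the Cylinder starts simulating physics.
; A looping timer then damages enemies tracked by Collision overlaps, without augmenting combo, until a tick limit clears it and hides the zone.
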(event OnComponentBeginOverlap(Collision)
  (params (OverlappedComponent :type Primitive%20Component%20Object%20Reference) (OtherActor :type Actor%20Object%20Reference) (OtherComp :type Primitive%20Component%20Object%20Reference) (OtherBodyIndex :type Integer) (bFromSweep :type Boolean) (SweepResult :type Hit%20Result%20Structure%20%28by%20ref%29))
  (bind _asbp_ennemi_parent (Utilities|Casting|CastToBP_EnnemiParent OtherActor))
  (Utilities|Array|Add (Variables|Default|GetEnnemisEnFeu) _asbp_ennemi_parent))

(event OnComponentEndOverlap(Collision)
  (params (OverlappedComponent :type Primitive%20Component%20Object%20Reference) (OtherActor :type Actor%20Object%20Reference) (OtherComp :type Primitive%20Component%20Object%20Reference) (OtherBodyIndex :type Integer))
  (bind _asbp_ennemi_parent (Utilities|Casting|CastToBP_EnnemiParent OtherActor))
  (Utilities|Array|RemoveItem (Variables|Default|GetEnnemisEnFeu) _asbp_ennemi_parent))

(event Custom|Incendie
  (bind _loopcount (Variables|Default|GetLoopCount))
  (for _array_element (Variables|Default|GetEnnemisEnFeu)
    (Default|HitTaken _array_element (Variables|Default|GetDamage) false))
  (if (>= _loopcount 20)
    (Utilities|Time|ClearandInvalidateTimerbyHandle (stale EventEnviroHit _returnvalue))
    (Rendering|SetVisibility (Variables|Default|GetCollision) false false)
    (else
      (Math|Integer|IncrementInt _loopcount))))

(event EventEnviroHit
  (params (PlayerRotation :type Rotator :default "0, 0, 0"))
  (Utilities|FlowControl|DoOnce false
    (:Completed
      (Transformation|SetActorRotation (Math|Rotator|MakeRotator (.roll PlayerRotation) (.pitch PlayerRotation) (+ (.yaw PlayerRotation) 1.8e+02)))
      (bind _barrelrotation (Timeline|Timeline PlayFromStart)
        (:Update
          (Transformation|SetRelativeRotation (Variables|Default|GetSphere) (Math|Rotator|MakeRotator 0.0 _barrelrotation 0.0) false false))
        (:Finished
          (Physics|SetSimulatePhysics (Variables|Default|GetCylinder) true)
          (Development|SetHiddeninGame (Variables|Default|GetCollision) false false)
          (bind _returnvalue (Utilities|Time|SetTimerbyEvent (delegate Custom|Incendie) 0.5 true)))))))

(fn ConstructionScript
  (|CallParentFunction))