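; BP_PoubelleTrap is an interactive trash can trap that tips over when hit and can release an enemy.
; On its first EnviroHit, it turns to the hitter's yaw plus 180 degrees, then a timeline pitches the Sphere component over.
; When the timeline finishes, the Cylinder starts simulating physics and, if SpawneUnEnnemi is set, an active BP_EnnemiD spawns at Sphere1.
; A comment marks a money drop for the false branch as still to do.
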(event EventBeginPlay
  (|CallParentFunction) ; This node is disabled and will not be called.\nDrag off pins to build functionality.
)

(event Collision|EventActorBeginOverlap
  (params (OtherActor :type Actor%20Object%20Reference))
  (|CallParentFunction OtherActor) ; This node is disabled and will not be called.\nDrag off pins to build functionality.
)

(event EventTick
  (params (DeltaSeconds :type Float%20%28single-precision%29))
  (|CallParentFunction DeltaSeconds) ; This node is disabled and will not be called.\nDrag off pins to build functionality.
)

(event EventEnviroHit
  (params (PlayerRotation :type Rotator :default "0, 0, 0"))
  (Utilities|FlowControl|DoOnce false
    (:Completed
      (Transformation|SetActorRotation (Math|Rotator|MakeRotator (.roll PlayerRotation) (.pitch PlayerRotation) (+ (.yaw PlayerRotation) 1.8e+02)))
      (bind _barrelrotation (Timeline|Timeline Play)
        (:Update
          (Transformation|SetRelativeRotation (Variables|Default|GetSphere) (Math|Rotator|MakeRotator 0.0 _barrelrotation 0.0) false false))
        (:Finished
          (Physics|SetSimulatePhysics (Variables|Default|GetCylinder) true)
          ;[1 1 1] Ajouter le drop d'argent sur le false
          (if (Variables|Default|GetSpawneUnEnnemi)
            (bind _returnvalue (Game|SpawnActorfromClass "/Game/EnnemiTest/EnnemiTest2/EnnemiDistance/BP_EnnemiD.BP_EnnemiD_C" (Transformation|GetWorldTransform (Variables|Default|GetSphere1)) "Undefined" "MultiplyWithRoot" 0 0))
            (Utilities|IsValid _returnvalue
              (:Is%20Valid
                (Variables|/Game/EnnemiTest/EnnemiTest2/BP_EnnemiParent.BP_EnnemiParent_C|SetIdlePause _returnvalue false)))))))))

(fn ConstructionScript
  (|CallParentFunction))