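; BP_Tornado is a damaging area actor that repeatedly hurts enemies caught inside its capsule.
; Capsule overlap events add and remove BP_EnnemiParent actors in the EnnemiInZone array.
; From BeginPlay, DealDamage calls HitTaken on each listed enemy without augmenting combo, then plays a world camera shake at the tornado's location.
; The event re-calls itself after a Delay of Duration, so that variable sets the interval between pulses.
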(event OnComponentBeginOverlap(Capsule)
  (params (OverlappedComponent :type Primitive%20Component%20Object%20Reference) (OtherActor :type Actor%20Object%20Reference) (OtherComp :type Primitive%20Component%20Object%20Reference) (OtherBodyIndex :type Integer) (bFromSweep :type Boolean) (SweepResult :type Hit%20Result%20Structure%20%28by%20ref%29))
  (bind _asbp_ennemi_parent (Utilities|Casting|CastToBP_EnnemiParent OtherActor))
  (Utilities|Array|Add (Variables|Default|GetEnnemiInZone) _asbp_ennemi_parent))

(event OnComponentEndOverlap(Capsule)
  (params (OverlappedComponent :type Primitive%20Component%20Object%20Reference) (OtherActor :type Actor%20Object%20Reference) (OtherComp :type Primitive%20Component%20Object%20Reference) (OtherBodyIndex :type Integer))
  (bind _asbp_ennemi_parent (Utilities|Casting|CastToBP_EnnemiParent OtherActor))
  (Utilities|IsValid _asbp_ennemi_parent
    (:Is%20Valid
      (Utilities|Array|RemoveItem (Variables|Default|GetEnnemiInZone) _asbp_ennemi_parent))))

(event Custom|DealDamage
  (Utilities|FlowControl|Sequence
    (:then_0
      (for _array_element (Variables|Default|GetEnnemiInZone)
        (Default|HitTaken _array_element (Variables|Default|GetDamage) false)))
    (:then_1
      (Camera|PlayWorldCameraShake "/Game/PRoject/PersoPrincipal/BP_CamShakeComboY.BP_CamShakeComboY_C" (Transformation|GetActorLocation) 0.0 1e+03)
      (Utilities|FlowControl|Delay (Variables|Default|GetDuration))
      (CallFunction|DealDamage))))

(event EventBeginPlay
  (CallFunction|DealDamage))

(fn ConstructionScript)