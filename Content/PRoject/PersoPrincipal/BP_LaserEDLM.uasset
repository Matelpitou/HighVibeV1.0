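; BP_LaserEDLM is a laser attack actor that repeatedly damages enemies inside its capsule for a limited lifetime.
; Capsule overlap events keep an array of the BP_EnnemiParent actors currently inside the beam.
; DealDamage calls HitTaken on each without augmenting combo, plays a camera shake, prints the enemy count, then re-triggers itself when the Delay timeline finishes.
; A separate lifetime timeline, started on BeginPlay, destroys the actor when it ends.
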(event OnComponentBeginOverlap(Capsule)
  (params (OverlappedComponent :type Primitive%20Component%20Object%20Reference) (OtherActor :type Actor%20Object%20Reference) (OtherComp :type Primitive%20Component%20Object%20Reference) (OtherBodyIndex :type Integer) (bFromSweep :type Boolean) (SweepResult :type Hit%20Result%20Structure%20%28by%20ref%29))
  (bind _asbp_ennemi_parent (Utilities|Casting|CastToBP_EnnemiParent OtherActor))
  (Utilities|Array|Add (Variables|Default|GetEnnemieInBox) _asbp_ennemi_parent))

(event OnComponentEndOverlap(Capsule)
  (params (OverlappedComponent :type Primitive%20Component%20Object%20Reference) (OtherActor :type Actor%20Object%20Reference) (OtherComp :type Primitive%20Component%20Object%20Reference) (OtherBodyIndex :type Integer))
  (bind _asbp_ennemi_parent (Utilities|Casting|CastToBP_EnnemiParent OtherActor))
  (Utilities|Array|RemoveItem (Variables|Default|GetEnnemieInBox) _asbp_ennemi_parent))

(event Custom|DealDamage
  (bind _ennemieinbox (Variables|Default|GetEnnemieInBox))
  (for _array_element _ennemieinbox
    (Default|HitTaken _array_element (Variables|Default|GetDamage) false))
  (Camera|PlayWorldCameraShake "/Game/PRoject/PersoPrincipal/BP_CamShakeEDLM.BP_CamShakeEDLM_C" (Transformation|GetWorldLocation (Variables|Default|GetDefaultSceneRoot)) 0.0 1e+03)
  (Development|PrintString (Utilities|String|ToString(Integer) (Utilities|Array|Length _ennemieinbox)))
  (Timeline|Delay PlayFromStart
    (:Finished
      (CallFunction|DealDamage))))

(event EventBeginPlay
  (Utilities|FlowControl|Sequence
    (:then_0
      (CallFunction|DealDamage))
    (:then_1
      (Timeline|Timeline PlayFromStart
        (:Finished
          (Actor|DestroyActor))))))

(fn ConstructionScript)