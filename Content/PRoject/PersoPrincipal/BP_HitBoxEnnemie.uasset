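; BP_HitBoxEnnemie is a short-lived hitbox actor that applies the player character's active damage to enemies it overlaps.
; On BeginPlay it caches the third-person player character, then destroys itself after a brief delay.
; Box overlaps call HitTaken on BP_EnnemiParent actors without augmenting the combo, or otherwise call EnviroHit on BP_Environment actors with the player's rotation.
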(event OnComponentBeginOverlap(Box)
  (params (OverlappedComponent :type Primitive%20Component%20Object%20Reference) (OtherActor :type Actor%20Object%20Reference) (OtherComp :type Primitive%20Component%20Object%20Reference) (OtherBodyIndex :type Integer) (bFromSweep :type Boolean) (SweepResult :type Hit%20Result%20Structure%20%28by%20ref%29))
  (bind _asbp_ennemi_parent (Utilities|Casting|CastToBP_EnnemiParent OtherActor)
    (:then
      (Default|HitTaken _asbp_ennemi_parent (Variables|/Game/PRoject/PersoPrincipal/BP_ThirdPersonCharacter.BP_ThirdPersonCharacter_C|GetDamageActif (Variables|Default|GetTPC)) false))
    (:CastFailed
      (bind _asbp_environment (Utilities|Casting|CastToBP_Environment OtherActor))
      (Default|EnviroHit _asbp_environment (Transformation|GetActorRotation (Variables|Default|GetTPC))))))

(event EventBeginPlay
  (bind _asbp_third_person_character (Utilities|Casting|CastToBP_ThirdPersonCharacter (Game|GetPlayerCharacter 0)))
  (Variables|Default|SetTPC _asbp_third_person_character)
  (Utilities|FlowControl|Delay 0.1)
  (Actor|DestroyActor))

(fn ConstructionScript)