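; Projectile VFX actor from an effects pack, with a trail effect and a separate impact effect.
; On BeginPlay it assigns its configured projectile and hit effect assets to the two effect components.
; When the collision sphere hits, it stops the trail, plays the hit effect at the impact point, disables collision, shakes the first player's camera and removes the light.
; The actor destroys itself after a delay.
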(event OnComponentHit(Sphere1)
  (params (HitComponent :type Primitive%20Component%20Object%20Reference) (OtherActor :type Actor%20Object%20Reference) (OtherComp :type Primitive%20Component%20Object%20Reference) (NormalImpulse :type Vector :default "0, 0, 0") (Hit :type Hit%20Result%20Structure%20%28by%20ref%29))
  (bind _hiteffects (Variables|Default|GetHiteffects))
  (Components|Activation|Deactivate (Variables|Default|GetProjectileEffect))
  (Components|Activation|SetActive _hiteffects true false)
  (Transformation|SetWorldLocation _hiteffects (.Location (Collision|BreakHitResult Hit)) false false)
  (Collision|SetCollisionEnabled (Variables|Default|GetSphere1) "NoCollision")
  (Game|Feedback|ClientStartCameraShake (Game|GetPlayerController 0) "/Game/Package/sA_Megapack_v1/sA_Projectilevfx/Vfx/Blueprints/BP_CameraShake01.BP_CameraShake01_C" (Variables|Default|GetCameraShakeStrength_Hit) "CameraLocal" "0, 0, 0")
  (Components|DestroyComponent (Variables|Default|GetPointLight))
  (Utilities|FlowControl|Delay 1e+01)
  (Actor|DestroyActor))

(event EventBeginPlay
  (Class|NiagaraComponent|SetAsset (Variables|Default|GetProjectileEffect) (Variables|Default|GetProjectilefx) true)
  (Class|NiagaraComponent|SetAsset (Variables|Default|GetHiteffects) (Variables|Default|GetHitEffect) true))

(fn ConstructionScript)