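; Quest NPC that turns toward the player when talked to and runs a step-based dialogue widget.
; Repeated Talk calls speed up or advance text, then close the widget, update the step and notify the character.
; UpdateGoal scans Vitres for failed or cleared entries, counting at most one clear per call, to set Failed or Completed.
; A MissionProgress RepNotify flags the quest finished when the goal is reached.
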(event Custom|UpdateGoal
  (for _array_element (Variables|Default|GetVitres)
    (if (Variables|/Game/NpcDialogueSystem/NPC_ConducteurTram/VitreTram.VitreTram_C|GetIsFailed _array_element)
      (Variables|Default|SetCurrentDialogueStep "Failed")
      (elif (Variables|/Game/NpcDialogueSystem/NPC_ConducteurTram/VitreTram.VitreTram_C|GetIsCleared _array_element)
        (Utilities|FlowControl|DoOnce false
          (:Completed
            (Math|Integer|IncrementInt (Variables|Default|GetMissionProgress)))))))
  (Utilities|FlowControl|Sequence
    (:then_0
      (Utilities|FlowControl|DoOnce false) ; enters at Reset
    )
    (:then_1
      (if (== (Variables|Default|GetMissionProgress) (Variables|Default|GetMissionGoal))
        (if (Utilities|Enum|NotEqual(Enum) (Variables|Default|GetCurrentDialogueStep) "Failed")
          (Variables|Default|SetCurrentDialogueStep "Completed"))))))

(event EventBeginPlay)

(event Collision|EventActorBeginOverlap
  (params (OtherActor :type Actor%20Object%20Reference)))

(event EventTick
  (params (DeltaSeconds :type Float%20%28single-precision%29)))

(event EventTalk
  (Transformation|SetActorRotation (Math|Rotator|MakeRotator 0.0 0.0 (.Yaw (Math|Rotator|BreakRotator (.rotation (Class|KismetAnimationLibrary|Lookat (Transformation|GetActorTransform) (Transformation|GetActorLocation (Game|GetPlayerCharacter 0)) (Transformation|GetActorLocation) false "0, 0, 0" 0.0))))))
  (if (Variables|Default|GetIsInDialogue)
    (if (Variables|/Game/NpcDialogueSystem/DialogueWidget.DialogueWidget_C|GetFinishedLine (stale _returnvalue))
      (if (Variables|/Game/NpcDialogueSystem/DialogueWidget.DialogueWidget_C|GetFinishedText (stale _returnvalue))
        (Variables|Default|SetIsInDialogue false)
        (if (Utilities|Enum|Equal(Enum) (Variables|Default|GetCurrentDialogueStep) "Intro")
          (Variables|Default|SetCurrentDialogueStep "Idle")
          (elif (Variables|Default|GetHasFinishedQuest)
            (Variables|Default|SetCurrentDialogueStep "Completed")))
        (Widget|RemovefromParent (stale _returnvalue))
        (bind _asbp_third_person_character (Utilities|Casting|CastToBP_ThirdPersonCharacter (Game|GetPlayerCharacter 0)))
        (Default|FinishDialogue _asbp_third_person_character)
        (else
          (Default|NextText (stale _returnvalue))))
      (else
        (Default|SpeedText (stale _returnvalue))))
    (else
      (Variables|Default|SetIsInDialogue true)
      (bind _returnvalue (UserInterface|CreateWidget "/Game/NpcDialogueSystem/DialogueWidget.DialogueWidget_C"))
      (Variables|/Game/NpcDialogueSystem/DialogueWidget.DialogueWidget_C|SetNPCName _returnvalue (Variables|Default|GetNPCName))
      (Variables|/Game/NpcDialogueSystem/DialogueWidget.DialogueWidget_C|SetCurrentStep _returnvalue (Variables|Default|GetCurrentDialogueStep))
      (UserInterface|Viewport|AddtoViewport _returnvalue 0)
      (Default|SetText _returnvalue))))

(fn ConstructionScript)

(fn OnRepMissionProgress
  (if (== (Variables|Default|GetMissionProgress) (Variables|Default|GetMissionGoal))
    (Variables|Default|SetHasFinishedQuest true)))